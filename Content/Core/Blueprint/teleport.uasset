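; Teleport trigger actor that moves anything entering its box to a target actor's location while swapping streamed levels.
; On box overlap it starts a non-blocking load of one level, sets the overlapping actor's transform from the target's location, then unloads another level.
; The overlapping actor is not filtered by type.
; The construction script writes a configurable label to a text render component.
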(event OnComponentBeginOverlap(Box)
  (params (OverlappedComponent :type Primitive%20Component%20Object%20Reference) (OtherActor :type Actor%20Object%20Reference) (OtherComp :type Primitive%20Component%20Object%20Reference) (OtherBodyIndex :type Integer) (bFromSweep :type Boolean) (SweepResult :type Hit%20Result%20Structure%20%28by%20ref%29))
  (Game|LoadStreamLevel(byName) (Variables|Default|GetLoadStream) true)
  (Transformation|SetActorLocationAndRotation OtherActor (Transformation|GetActorLocation (Variables|Default|GetNewVar_0)))
  (Game|UnloadStreamLevel(byName) (Variables|Default|GetUnlound)))

(event EventBeginPlay)

(event Collision|EventActorBeginOverlap
  (params (OtherActor :type Actor%20Object%20Reference)))

(event EventTick
  (params (DeltaSeconds :type Float%20%28single-precision%29)))

(fn ConstructionScript
  (Rendering|Components|TextRender|SetText (Variables|Default|GetTextRender) (Variables|Default|GetText)))